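; Attack component that provides a lightning strike and a targeted heal, both built on spawned AoE actors.
; LightningStrike spawns a delayed strike that ignores its instigator; overlapped actors receive a damage message, and successful damage spawns a damage display at the attack target.
; HealTarget line-traces downward from the target to place and trigger a timed heal AoE, whose overlap callback heals only that target.
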(event `LightningStrike`
  (params (DelayBeforeStrike :type "Float (single-precision)") (AttackTarget :type "Actor Object Reference") (DamageAmount :type "Float (double-precision)"))
  (bind (_aspawn _bsuccess) (cast `Pawn` (`self.GetOwner`) :!pure true))
  (bind _returnvalue (`|SpawnActorFromClass` "/Game/AoE/BP_AoE_LightningStrike.BP_AoE_LightningStrike_C" (`KismetMathLibrary.MakeTransform` (0.0 0.0 0.0)) "Undefined" "MultiplyWithRoot" null DelayBeforeStrike AttackTarget true false false (select `bool` _bsuccess :`false` _aspawn)))
  (add `/Game/AoE/BP_AoE_Base.OnAOEOverlapActor` _returnvalue (delegate `DamageAoE`)))

(event `DamageAoE`
  (params (Actor :type "Actor Object Reference"))
  (bind _wasdamaged (message `/Game/DamageSystem/BPI_Damagable.TakeDamage` Actor (stale `LightningStrike` DamageAmount)))
  (if _wasdamaged
    (`|SpawnActorFromClass` "/Game/UI/DamageDisplay/BP_DamageDisplay.BP_DamageDisplay_C" (`KismetMathLibrary.Conv_VectorToTransform` (`Actor.K2_GetActorLocation` (stale `LightningStrike` AttackTarget))) "Undefined" "MultiplyWithRoot" null (stale `LightningStrike` DamageAmount) null)))

(event `HealTarget`
  (params (HealTarget :type "Actor Object Reference"))
  (bind _returnvalue (`Actor.K2_GetActorLocation` HealTarget))
  (`/Engine/EditorBlueprintResources/StandardMacros.IsValid` HealTarget
    (:`Is Valid`
      (bind (_outhit _returnvalue_2) (`KismetSystemLibrary.LineTraceSingle` _returnvalue (* _returnvalue (1.0 1.0 -1000.0)) "TraceTypeQuery1" false (`|MakeArray` HealTarget)))
      (if _returnvalue_2
        (bind _returnvalue_3 (`|SpawnActorFromClass` "/Game/AoE/BP_AoE_Heal.BP_AoE_Heal_C" (`KismetMathLibrary.MakeTransform` (`.Location` (`GameplayStatics.BreakHitResult` _outhit))) "Undefined" "MultiplyWithRoot" null 1.0 10.0 false false false null))
        (add `/Game/AoE/BP_AoE_Base.OnAOEOverlapActor` _returnvalue_3 (delegate `OnHealTarget`))
        (`/Game/AoE/BP_AoE_Base.Trigger` _returnvalue_3)))))

(event `OnHealTarget`
  (params (Actor :type "Actor Object Reference"))
  (if (== Actor (stale `HealTarget` HealTarget))
    (message `/Game/DamageSystem/BPI_Damagable.Heal` Actor 10.0)))