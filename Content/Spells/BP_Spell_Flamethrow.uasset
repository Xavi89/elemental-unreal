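; Flamethrower spell actor whose box collision grows along a timeline from BeginPlay, forming the damage area.
; Overlapping actors other than the owner receive a small fixed damage message, and a successful result spawns a damage number display at the impact point.
; A separate Hit event plays explosion particles and sound at the given location, then destroys the spell; nothing in this graph calls it.
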(event `self.ReceiveHit`
  (params (MyComp :type "PrimitiveComponent Object Reference") (Other :type "Actor Object Reference") (OtherComp :type "PrimitiveComponent Object Reference") (bSelfMoved :type Boolean) (HitLocation :type "Vector Structure") (HitNormal :type "Vector Structure") (NormalImpulse :type "Vector Structure") (Hit :type "HitResult Structure (by ref)"))
  (`GameplayStatics.SpawnEmitterAtLocation` "/Game/StarterContent/Particles/P_Explosion.P_Explosion" HitLocation)
  (`GameplayStatics.PlaySoundAtLocation` "/Game/StarterContent/Audio/Explosion_Cue.Explosion_Cue" HitLocation (struct) 1.0 1.0 0.0 null null null null)
  (`/Engine/EditorBlueprintResources/StandardMacros.IsValid` self
    (:`Is Valid`
      (`self.K2_DestroyActor`))))

(event `self.ReceiveBeginPlay`
  (bind (_direction _scale) (`Timeline|ScaleUp` :!via `PlayFromStart`)
    (:`Update`
      (`SceneComponent.SetRelativeScale3D` (`self.BoxCollision`) (`KismetMathLibrary.Conv_DoubleToVector` _scale)))))

(event `self.BoxCollision.OnComponentBeginOverlap`
  (params (OverlappedComponent :type "PrimitiveComponent Object Reference") (OtherActor :type "Actor Object Reference") (OtherComp :type "PrimitiveComponent Object Reference") (OtherBodyIndex :type Integer) (bFromSweep :type Boolean) (SweepResult :type "HitResult Structure (by ref)"))
  (bind _s_damageinfo (make `/Game/DamageSystem/S_DamageInfo` 3.0 "NewEnumerator1"))
  (bind (_amount _school) (break `/Game/DamageSystem/S_DamageInfo` _s_damageinfo))
  (if (!= OtherActor (`self.GetOwner`))
    (bind _wasdamaged (message `/Game/DamageSystem/BPI_Damagable.TakeDamage` OtherActor _s_damageinfo))
    (if _wasdamaged
      (`|SpawnActorFromClass` "/Game/UI/DamageDisplay/BP_DamageDisplay.BP_DamageDisplay_C" (`KismetMathLibrary.Conv_VectorToTransform` (`.ImpactPoint` (`GameplayStatics.BreakHitResult` SweepResult))) "Undefined" "MultiplyWithRoot" null _amount _school null))))

(fn `UserConstructionScript`
  (`parent.UserConstructionScript`))