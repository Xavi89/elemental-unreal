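; Base projectile actor for spells, which flies toward an optional target and destroys itself on impact or after a short lifetime.
; The construction script applies speed and gravity to the projectile movement and enables homing when a valid target is set.
; BeginPlay makes the box collision ignore the owner and aims velocity at the target.
; Hits fire an OnSpellImpact dispatcher and spawn impact effect and sound.
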(event `self.ReceiveBeginPlay`
  (`|ExecutionSequence`
    (:`then_0`
      (`KismetSystemLibrary.Delay` 5.0)
      (`/Engine/EditorBlueprintResources/StandardMacros.IsValid` self
        (:`Is Valid`
          (`self.K2_DestroyActor`))))
    (:`then_1`
      (`PrimitiveComponent.IgnoreActorWhenMoving` (`self.BoxCollision`) (`self.GetOwner`) true)
      (`self.Target`
        (:`then`
          (`self.RotateToTarget`))
        (:`else`)))))

(event `RotateToTarget`
  (set `MovementComponent.Velocity` (* (`KismetMathLibrary.GetDirectionUnitVector` (`self.K2_GetActorLocation`) (`self.K2_GetActorLocation` (`self.Target`))) (`self.Speed`)) (`self.ProjectileMovement`)))

(event `self.BoxCollision.OnComponentHit`
  (params (HitComponent :type "PrimitiveComponent Object Reference") (OtherActor :type "Actor Object Reference") (OtherComp :type "PrimitiveComponent Object Reference") (NormalImpulse :type "Vector Structure") (Hit :type "HitResult Structure (by ref)"))
  (bind (_bblockinghit _binitialoverlap _time _distance _location) (`GameplayStatics.BreakHitResult` Hit))
  (`self.OnSpellImpact` OtherActor Hit)
  (`GameplayStatics.SpawnEmitterAtLocation` (`self.ImpactEffect`) _location)
  (`GameplayStatics.PlaySoundAtLocation` (`self.ImpactSound`) _location (struct) 1.0 1.0 0.0 null null null null)
  (`/Engine/EditorBlueprintResources/StandardMacros.IsValid` self
    (:`Is Valid`
      (`self.K2_DestroyActor`))))

(fn `UserConstructionScript`
  (bind _projectilemovement (`self.ProjectileMovement`))
  (set `ProjectileMovementComponent.InitialSpeed` (`self.Speed`) _projectilemovement)
  (set `ProjectileMovementComponent.MaxSpeed` (`self.Speed`) _projectilemovement)
  (set `ProjectileMovementComponent.ProjectileGravityScale` (`self.Gravity`) _projectilemovement)
  (set `self.Damage` (`self.Damage`))
  (`self.Target`
    (:`then`
      (if (`self.IsHoming`)
        (set `ProjectileMovementComponent.bIsHomingProjectile` true _projectilemovement)
        (set `ProjectileMovementComponent.HomingTargetComponent` (`Actor.RootComponent` (`self.Target`)) _projectilemovement)))
    (:`else`)))